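; BP_CameraC is a work-in-progress camera Blueprint with a spring arm, apparently intended for pinch zoom.
; Its touch input only prints a debug message; other events are empty or unreachable.
; GetTouchDistance measures the gap between two touches, or uses the mouse position's length on Windows.
; A zoom macro stores that distance and arm length, but its viewport-scaled zoom math is left unconnected.
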(event `self.ReceiveBeginPlay`)

(event `EnhancedInput|/Game/IWP/Camera/IA_CameraC`
  (params (ActionValue :type Boolean) (ElapsedSeconds :type "Float (double-precision)") (TriggeredSeconds :type "Float (double-precision)") (InputAction :type "InputAction Object Reference" :default "/Game/IWP/Camera/IA_CameraC.IA_CameraC")))

(event `EnhancedInput|/Game/TopDown/Input/Actions/IA_SetDestination_Touch`
  (params (ActionValue :type Boolean) (ElapsedSeconds :type "Float (double-precision)") (TriggeredSeconds :type "Float (double-precision)") (InputAction :type "InputAction Object Reference" :default "/Game/TopDown/Input/Actions/IA_SetDestination_Touch.IA_SetDestination_Touch"))
  (:`Triggered`
    (`KismetSystemLibrary.PrintString` "Hello")))

(fn `Get Touch Distance`
  (returns (`Touch Distance` :type "Float (double-precision)"))
  (bind _returnvalue (`GameplayStatics.GetPlayerController` 0))
  (bind (_locationx _locationy) (`PlayerController.GetInputTouchState` _returnvalue "Touch2"))
  (bind (_locationx_2 _locationy_2) (`PlayerController.GetInputTouchState` _returnvalue "Touch1"))
  (bind (_locationx_3 _locationy_3) (`PlayerController.GetMousePosition` _returnvalue))
  (return (`KismetMathLibrary.VSize2D` (select `bool` (`KismetStringLibrary.EqualEqual_StrStr` (`GameplayStatics.GetPlatformName`) "Windows") :`false` (- (`KismetMathLibrary.MakeVector2D` _locationx_2 _locationy_2) (`KismetMathLibrary.MakeVector2D` _locationx _locationy)) :`true` (`KismetMathLibrary.MakeVector2D` _locationx_3 _locationy_3)))))

(fn `UserConstructionScript`)