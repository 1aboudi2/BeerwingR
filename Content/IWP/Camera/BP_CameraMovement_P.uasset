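; BP_CameraMovement_P is a camera Blueprint with an unfinished pinch-to-zoom for its spring arm.
; The IA_DRAG input prints debug text and sets arm length from pinchCmaeraZoom, but the node that updates that variable is unconnected.
; GetTouchDistance measures the gap between two touches, or the mouse position's vector length on Windows.
; The pinch graph caches touch and arm distances, leaving its viewport-scaled zoom delta unused.
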(event Input|EnhancedActionEvents|EnhancedInputActionIA_DRAG_
  (params (ActionValue :type Boolean) (ElapsedSeconds :type Float%20%28double-precision%29) (TriggeredSeconds :type Float%20%28double-precision%29) (InputAction :type Input%20Action%20Object%20Reference :default "/Game/TopDown/Input/Actions/IA_DRAG_.IA_DRAG_"))
  (Development|PrintText "Hello")
  (Development|PrintString (Utilities|String|ToString(Float) (stale _touch_distance)))
  (Variables|/Script/Engine.SpringArmComponent|SetTargetArmLength (Variables|Default|GetSpringArm) (stale _touch_distance)))

(fn ConstructionScript)

(fn GetTouchDistance
  (bind _returnvalue (Game|GetPlayerController 0))
  (bind (_locationx _locationy) (Class|PlayerController|GetInputTouchState _returnvalue "Touch2"))
  (bind (_locationx_2 _locationy_2) (Class|PlayerController|GetInputTouchState _returnvalue "Touch1"))
  (bind (_locationx_3 _locationy_3) (Game|Player|GetMousePosition _returnvalue))
  (return (Math|Vector2D|Vector2DLength (select (Utilities|Enum|Equal(Enum) (Game|GetPlatformName) "Windows") (Math|Vector2D|MakeVector2D _locationx_3 _locationy_3) (- (Math|Vector2D|MakeVector2D _locationx_2 _locationy_2) (Math|Vector2D|MakeVector2D _locationx _locationy))))))