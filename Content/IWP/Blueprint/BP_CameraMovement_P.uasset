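; BP_CameraMovement_P is an unfinished pinch-zoom camera prototype meant to drive a SpringArm's arm length.
; GetTouchDistance returns the distance between two touches, or the mouse position's vector length on Windows.
; PinchCmaeraZoom caches that distance and the current arm length, but its viewport-scaled zoom math is unconnected.
; The EventGraph chains that would apply the zoom and print debug text never run.
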(fn `Get Touch Distance`
  (returns (`Touch Distance` :type "Float (double-precision)"))
  (bind _returnvalue (`GameplayStatics.GetPlayerController` 0))
  (bind (_locationx _locationy) (`PlayerController.GetInputTouchState` _returnvalue "Touch2"))
  (bind (_locationx_2 _locationy_2) (`PlayerController.GetInputTouchState` _returnvalue "Touch1"))
  (bind (_locationx_3 _locationy_3) (`PlayerController.GetMousePosition` _returnvalue))
  (return (`KismetMathLibrary.VSize2D` (select `bool` (`KismetStringLibrary.EqualEqual_StrStr` (`GameplayStatics.GetPlatformName`) "Windows") :`false` (- (`KismetMathLibrary.MakeVector2D` _locationx_2 _locationy_2) (`KismetMathLibrary.MakeVector2D` _locationx _locationy)) :`true` (`KismetMathLibrary.MakeVector2D` _locationx_3 _locationy_3)))))

(fn `UserConstructionScript`)