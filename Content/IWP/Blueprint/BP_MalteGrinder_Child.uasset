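; BP_MalteGrinder_Child is a malt grinder asset that extends a parent grinder Blueprint with its own display text and grind setting.
; On BeginPlay it runs the parent logic, then sets the asset's title and information strings.
; Every Tick it polls the GrindSlider in the malt grinder widget and stores the result in GrindValue.
; Construction only calls the parent script.
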(event `self.ReceiveBeginPlay`
  (`parent.ReceiveBeginPlay`)
  (set `self.AssetTitleGrind` "MaltGrider1")
  (set `self.AssetInformation` "Ready to gride soeme beans?!"))

(event `self.ReceiveTick`
  (params (DeltaSeconds :type "Float (single-precision)"))
  (`parent.ReceiveTick` DeltaSeconds)
  (set `self.grindValue` (`Slider.GetValue` (`/Game/IWP/Blueprint/Widgets/WP_MaltGrinderInformation.GrindSlider` (`self.AssetMaltGrinderWidget`)))))

(fn `UserConstructionScript`
  (`parent.UserConstructionScript`))