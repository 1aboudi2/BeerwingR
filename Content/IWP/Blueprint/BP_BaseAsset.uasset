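; Base actor for placeable beer-production buildings, with a touch-opened information menu and beer fluid storage and transfer.
; BeginPlay creates confirm and information widgets, binds placeholder start/stop and transfer handlers for children, and follows build-mode dispatchers, which suppress the menu while building.
; TransferBeerFluid offers its fluid to actors of a given class until one empty receiver accepts, then clears itself.
; Helpers swap in a preview material, and a debug button toggles test fluid.
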(event `self.ReceiveTick`
  (params (DeltaSeconds :type "Float (single-precision)"))
  (`/Engine/EditorBlueprintResources/StandardMacros.IsValid` (`self.widget`)))

(event `self.ReceiveBeginPlay`
  (bind _returnvalue (`|CreateWidget` "/Game/IWP/Blueprint/Widgets/WP_ConfirmBuild.WP_ConfirmBuild_C"))
  (bind _output_get (set `self.ConfirmMenu` _returnvalue))
  (`UserWidget.AddToViewport` _output_get 0)
  (bind _returnvalue_2 (`|CreateWidget` "/Game/IWP/Blueprint/Widgets/WP_AssetInformation.WP_AssetInformation_C"))
  (bind _output_get_2 (set `self.AssetInformationWidget` _returnvalue_2))
  (`UserWidget.AddToViewport` _output_get_2 0)
  (add `/Game/IWP/Blueprint/Widgets/WP_AssetInformation.StartStopButtonDispatcher` (`self.AssetInformationWidget`) (delegate `StartStopButton`)) ; Bind Event to button in Asset Information. This event will be caled if button is pressed
  (add `/Game/IWP/Blueprint/Widgets/WP_AssetInformation.TransferButtonDispatcher` (`self.AssetInformationWidget`) (delegate `TransferButton`))
  ;[0.08239 1 0.2273] Link the asset to building mode toggle using event dispatchers
  (bind _foundwidgets (`WidgetBlueprintLibrary.GetAllWidgetsOfClass` "/Game/IWP/Blueprint/Widgets/WP_BuildingMenu.WP_BuildingMenu_C" false))
  (bind _output_get_3 (set `self.BuildingMenu` (`|GetArrayItem` _foundwidgets)))
  (add `/Game/IWP/Blueprint/Widgets/WP_BuildingMenu.BuildModeOff` _output_get_3 (delegate `SetBuildingFalse`))
  (add `/Game/IWP/Blueprint/Widgets/WP_BuildingMenu.BuildModeOn` _output_get_3 (delegate `SetBuildingTrue`))
  (add `/Game/IWP/Blueprint/Widgets/WP_AssetInformation.DebugCreateBeerDispatcher` (`self.AssetInformationWidget`) (delegate `DebugCreateBeer`)))

(event `StartStopButton`
  (`KismetSystemLibrary.PrintString` "Start Stop clicked"))

(event `DebugCreateBeer`
  (`/Engine/EditorBlueprintResources/StandardMacros.IsValid` (`self.BeerFluid`)
    (:`Is Valid`
      (`self.ClearBeerFluid`))
    (:`Is Not Valid`
      (bind _returnvalue (`|GenericCreateObject` "/Game/IWP/Blueprint/BP_BeerFluid.BP_BeerFluid_C"))
      (set `self.BeerFluid` _returnvalue)
      (set `self.BeerFluidAmount` 1.0)
      (`KismetSystemLibrary.PrintString` "added Water"))))

(event `TransferButton`
  (`KismetSystemLibrary.PrintString` "Transfer button clicked"))

(event `SetBuildingTrue`
  ;[0.08239 1 0.2273] Link the asset to building mode toggle using event dispatchers
  (set `self.BuildingMode?` true)
  (`KismetSystemLibrary.PrintString` "canBuild"))

(event `SetBuildingFalse`
  ;[0.08239 1 0.2273] Link the asset to building mode toggle using event dispatchers
  (set `self.BuildingMode?` false)
  (`KismetSystemLibrary.PrintString` "cannotBuild"))

(event `self.FakeAssetCube.OnInputTouchEnd`
  (params (FingerIndex :type "ETouchIndex Enum" :default "Touch1") (TouchedComponent :type "PrimitiveComponent Object Reference"))
  (bind _assetinformationwidget (`self.AssetInformationWidget`))
  (if (`self.BuildingMode?`)
    (`KismetSystemLibrary.PrintString` "building true")
    (elif (`self.Clicked`)
      (set `self.Clicked` false)
      (`KismetSystemLibrary.PrintString` "unclicked")
      (else
        (set `self.Clicked` true)
        (`/Game/IWP/Blueprint/Widgets/WP_AssetInformation.Asset menu` (`self.AssetInformationWidget`))
        (set `TextBlock.Text` (`self.AssetTitle`) (`/Game/IWP/Blueprint/Widgets/WP_AssetInformation.AssetTitle` _assetinformationwidget))
        (set `TextBlock.Text` (`self.AssetInformation`) (`/Game/IWP/Blueprint/Widgets/WP_AssetInformation.AssetInformation` _assetinformationwidget))))))

(event `Key|LeftMouseButton`
  (params (Key :type "Key Structure"))
  (:`Pressed`
    (`KismetSystemLibrary.PrintString` "click")))

(fn `Change Material`
  (set `self.BaseAssetMaterial` (`PrimitiveComponent.GetMaterial` (`self.FakeAssetCube`) 0))
  (`PrimitiveComponent.SetMaterial` (`self.FakeAssetCube`) 0 "/Game/IWP/Assets/Materials/Placeholder/M_Preview.M_Preview"))

(fn `CleanBuilding`)

(fn `ClearBeerFluid`
  (set `self.BeerFluid` null)
  (set `self.BeerFluidAmount` 0.0))

(fn `ReceiveBeerFluid`
  (params (IncomingBeerFluid :type "/Game/IWP/Blueprint/BP_BeerFluid Object Reference") (FluidAmount :type "Float (double-precision)"))
  (returns (Accpeted :type Boolean))
  (if (`self.isBeerReceiver`)
    (if (`KismetSystemLibrary.IsValid` (`self.BeerFluid`))
      _
      (else
        (set `self.BeerFluid` IncomingBeerFluid)
        (set `self.BeerFluidAmount` (`local.FluidAmount`))
        (return true) ; Return true after the builign accepted the new fluid
      ))
    (else
      (`KismetSystemLibrary.PrintString` "Trying to send to non beer receiver")))
  (return false) ; Return false if building doesnt accept fluids or already has one
)

(fn `Reset Material`
  (`PrimitiveComponent.SetMaterial` (`self.FakeAssetCube`) 0 (`self.BaseAssetMaterial`)))

(fn `TransferBeerFluid`
  (params (TargetClass :type "/Game/IWP/Blueprint/BP_BaseAsset Class Reference"))
  (if (`KismetSystemLibrary.IsValid` (`self.BeerFluid`))
    (`KismetSystemLibrary.PrintString` "Searching for targets to transfer beer to")
    (bind _outactors (`GameplayStatics.GetAllActorsOfClass` TargetClass))
    (for _array_element _outactors
      (bind _accpeted (`self.ReceiveBeerFluid` _array_element (`self.BeerFluid`) (`self.BeerFluidAmount`)))
      (if _accpeted
        (`self.ClearBeerFluid`)
        (`KismetSystemLibrary.PrintString` "Transfered beer to")
        (`KismetSystemLibrary.PrintString` (`KismetSystemLibrary.GetClassDisplayName` TargetClass))
        (break)
        (else
          (`KismetSystemLibrary.PrintString` "transfer target did not accept"))))
    (`KismetSystemLibrary.PrintString` "finished searching")
    (else
      (`KismetSystemLibrary.PrintString` "Currently no fluid present"))))

(fn `UserConstructionScript`)