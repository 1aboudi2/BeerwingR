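; Grid placement actor that snaps BP_FakeAssetChild actors to cells under the mouse cursor.
; Each tick it traces under the cursor, checks bounds and converts the hit to an index in a boolean occupancy array.
; On free cells it alternates between snapping the held Machine and releasing it, or spawning a replacement and marking the cell occupied.
; BP_Tile generation and touch tracing exist but are not used by the event graph.
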(event `self.ReceiveBeginPlay`
  (bind _returnvalue (`|SpawnActorFromClass` "/Game/IWP/Blueprint/BP_FakeAssetChild.BP_FakeAssetChild_C" (`KismetMathLibrary.MakeTransform` (0.0 0.0 0.0)) "AlwaysSpawn" "MultiplyWithRoot" null null))
  (set `self.Machine` _returnvalue)
  (`self.InitializeTilesBool`))

(event `self.ReceiveTick`
  (params (DeltaSeconds :type "Float (single-precision)"))
  (bind (_hit _location) (`self.Get Location Mouse`))
  (bind (_leftbottomv_x _leftbottomv_y) (`KismetMathLibrary.BreakVector` (`self.LeftBottomV`)))
  (bind (_righttopv_x _righttopv_y) (`KismetMathLibrary.BreakVector` (`self.RightTopV`)))
  (bind _returnvalue (`KismetMathLibrary.MakeVector` (.x _location) (.y _location)))
  (`|ExecutionSequence`
    (:`then_0`
      (if _hit
        (if (or (< (.x _location) _leftbottomv_x) (> (.x _location) _righttopv_x) (< (.y _location) _leftbottomv_y) (> (.y _location) _righttopv_y))
          (`KismetSystemLibrary.PrintString` (`KismetStringLibrary.Conv_VectorToString` _returnvalue) true true (struct :`G` 0.66 :`B` 1.0 :`A` 1.0) 4.0)
          (else
            (bind _index (`self.GetIndexFromPos` (.x _location) (.y _location)))
            (if (not (`|GetArrayItem` (`self.isTileOccupied`) _index))
              (`KismetSystemLibrary.PrintString` (`KismetStringLibrary.Conv_IntToString` _index))
              (bind _machine (`self.Machine`)
                (:`then`
                  (`SceneComponent.K2_SetWorldLocation` (`Actor.RootComponent` _machine) (`self.Get Grid Location` _returnvalue) false false)
                  (set `self.Machine` null))
                (:`else`
                  (bind _returnvalue_2 (`|SpawnActorFromClass` "/Game/IWP/Blueprint/BP_FakeAssetChild.BP_FakeAssetChild_C" (`KismetMathLibrary.MakeTransform` (0.0 0.0 0.0)) "AlwaysSpawn" "MultiplyWithRoot" null null))
                  (set `self.Machine` _returnvalue_2)
                  (`KismetArrayLibrary.Array_Set` (`self.isTileOccupied`) _index true))))))))))

(fn `ClearTiles`
  (bind _tiles (`self.Tiles`))
  (if (> (`KismetArrayLibrary.Array_Length` _tiles) 0)
    (for _array_element _tiles
      (`self.K2_DestroyActor` _array_element))
    (`KismetArrayLibrary.Array_Clear` _tiles)
    (else
      (for _array_element_2 (`self.Tiles`)
        (`KismetSystemLibrary.PrintString` (`KismetSystemLibrary.GetDisplayName` _array_element_2))))))

(fn `Get Grid Location`
  (params (Location :type "Vector Structure"))
  (returns (LocationOnGrid :type "Vector Structure"))
  (bind _gridsize (`self.gridSize`))
  (bind _returnvalue (/ _gridsize 2.0))
  (return (`KismetMathLibrary.MakeVector` (+ (* (`KismetMathLibrary.Conv_IntToDouble` (`KismetMathLibrary.Round` (/ (- Location_X _returnvalue) _gridsize))) _gridsize) _returnvalue) (+ (* (`KismetMathLibrary.Conv_IntToDouble` (`KismetMathLibrary.Round` (/ (- Location_Y _returnvalue) _gridsize))) _gridsize) _returnvalue))))

(fn `Get Location Finger`
  (returns (Hit :type Boolean) (Location :type "Vector Structure"))
  (bind (_bblockinghit _binitialoverlap _time _distance _location) (`GameplayStatics.BreakHitResult` (`PlayerController.GetHitResultUnderFingerByChannel` (`GameplayStatics.GetPlayerController` 0) "Touch1" "TraceTypeQuery1" true)))
  (return _bblockinghit _location))

(fn `Get Location Mouse`
  (returns (Hit :type Boolean) (Location :type "Vector Structure"))
  (bind (_bblockinghit _binitialoverlap _time _distance _location) (`GameplayStatics.BreakHitResult` (`PlayerController.GetHitResultUnderCursorByChannel` (`GameplayStatics.GetPlayerController` 0) "TraceTypeQuery1" true)))
  (return _bblockinghit _location))

(fn `GetIndexFromPos`
  (params (x :type "Float (double-precision)") (y :type "Float (double-precision)"))
  (returns (index :type Integer))
  (return (+ (`KismetMathLibrary.FFloor` (/ x (`self.TileSize`))) (* (`self.matrixRow`) (`KismetMathLibrary.FFloor` (/ y (`self.TileSize`)))))))

(fn `InitializeTiles`
  (`self.ClearTiles`)
  (for _index (range (`self.matrixRow`))
    (for _index_2 (range (`self.matrixColumn`))
      (bind _returnvalue (`|SpawnActorFromClass` "/Game/IWP/Blueprint/BP_Tile.BP_Tile_C" (`KismetMathLibrary.MakeTransform` (`self.K2_GetActorLocation`) (`self.K2_GetActorRotation`)) "AlwaysSpawn" "MultiplyWithRoot" self _index_2 _index null))
      (`/Game/IWP/Blueprint/BP_Tile.InitializeTile` _returnvalue)
      (bind _returnvalue_2 (`KismetArrayLibrary.Array_Add` (`self.Tiles`) _returnvalue))
      (set `/Game/IWP/Blueprint/BP_Tile.PosInArray` _returnvalue_2 _returnvalue))))

(fn `InitializeTilesBool`
  (bind _matrixcolumn (`self.matrixColumn`))
  (for _index (range (`self.matrixRow`))
    (for _index_2 (range _matrixcolumn)
      (`KismetArrayLibrary.Array_Set` (`self.isTileOccupied`) (+ _index_2 (* _index _matrixcolumn)) false true))))

(fn `New Matrix`
  (params (Length :type Integer) (Width :type Integer)))

(fn `UserConstructionScript`)