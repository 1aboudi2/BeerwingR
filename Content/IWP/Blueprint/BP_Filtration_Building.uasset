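; Filtration Tank building that receives beer and filters out malt pieces.
; Tick advances filtration by the UI speed slider, building malt residuals and pump clogging, which halts processing when full.
; Idle residuals rot into contamination, passed to beer on start; cleaning the pump with beer inside applies a fluid loss.
; Completion shows a transfer popup that only logs and hides; the transfer button sends beer to BP_CookingTank.
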(event `self.ReceiveBeginPlay`
  (`parent.ReceiveBeginPlay`)
  (set `self.isBeerReceiver` true)
  (set `self.AssetTitle` "Filtration Tank")
  (set `self.AssetInformation` "Filter out malt pieces")
  (add `/Game/IWP/Blueprint/Widgets/WP_AssetInformation.CleanFilterButtonDispatcher` (`self.AssetInformationWidget`) (delegate `CleanFilterButton`))
  (`Widget.SetVisibility` (`/Game/IWP/Blueprint/Widgets/WP_AssetInformation.FilterSpeedContainer` (`self.AssetInformationWidget`)) "SelfHitTestInvisible")
  (`Widget.SetVisibility` (`/Game/IWP/Blueprint/Widgets/WP_AssetInformation.FilterPumpContainer` (`self.AssetInformationWidget`)) "SelfHitTestInvisible")
  (`Widget.SetVisibility` (`/Game/IWP/Blueprint/Widgets/WP_AssetInformation.Start-Stop_ButtonContainer` (`self.AssetInformationWidget`)) "SelfHitTestInvisible")
  (`Widget.SetVisibility` (`/Game/IWP/Blueprint/Widgets/WP_AssetInformation.TransferContainer` (`self.AssetInformationWidget`)) "SelfHitTestInvisible")
  ;[0.4702 0.01995 1] Transfering Liquids
  (bind _aswp_transfer_popup (cast `/Game/IWP/Blueprint/Widgets/WP_Transfer_Popup` (`WidgetComponent.GetWidget` (`self.WP_Transfer_Popup`))))
  (add `/Game/IWP/Blueprint/Widgets/WP_Transfer_Popup.TransferReady_Popup_Pressed` _aswp_transfer_popup (delegate `TransferLquid`))
  (`SceneComponent.SetVisibility` (`self.WP_Transfer_Popup`) false false))

(event `TransferLquid`
  ;[0.4702 0.01995 1] Transfering Liquids
  (`KismetSystemLibrary.PrintString` "Transferred Liquid Filtration" true true (struct :`G` 0.185822 :`B` 1.0 :`A` 1.0))
  (`SceneComponent.SetVisibility` (`self.WP_Transfer_Popup`) false false))

(event `CleanFilterButton`
  (`self.CleanPump`)
  (`self.UpdatePumpStatusText`))

(event `self.StartStopButton`
  (bind _beerfluid (`self.BeerFluid`))
  (`parent.StartStopButton`)
  (if (`KismetSystemLibrary.IsValid` (`self.BeerFluid`))
    (if (`self.isProcessing`)
      (`KismetSystemLibrary.PrintString` "Already processing")
      (elif (< (`self.CloggingLevel`) 1.0)
        (set `self.isProcessing` true) ; Add check that it cant start with clogged pump
        (if (> (`self.Contamination`) 0.0)
          (set `/Game/IWP/Blueprint/BP_BeerFluid.Contamination` (+ (`/Game/IWP/Blueprint/BP_BeerFluid.Contamination` _beerfluid) (`self.Contamination`)) _beerfluid)
          (`KismetArrayLibrary.Array_Add` (`/Game/IWP/Blueprint/BP_BeerFluid.FailLog` _beerfluid) "Filtering in contaminated tank contaminated the beer")
          (set `self.IdleTime` 0.0))
        (else
          (`KismetSystemLibrary.PrintString` "Trying to start with clogged pump"))))
    (else
      (`KismetSystemLibrary.PrintString` "Starting filtration with no beer fluid" true true (struct :`R` 1.0 :`B` 0.11617 :`A` 1.0)))))

(event `self.ReceiveTick`
  (params (DeltaSeconds :type "Float (single-precision)"))
  (bind _beerfluid (`self.BeerFluid`))
  (bind _beerfluid_2 (`self.BeerFluid`))
  (bind _maltclumpscontent (`/Game/IWP/Blueprint/BP_BeerFluid.MaltClumpsContent` _beerfluid_2))
  (bind _returnvalue (`Slider.GetValue` (`/Game/IWP/Blueprint/Widgets/WP_AssetInformation.FilterSpeedSlider` (`self.AssetInformationWidget`))))
  (bind _returnvalue_2 (* DeltaSeconds (`self.FilteringEfficiency`) (`Slider.GetValue` (`/Game/IWP/Blueprint/Widgets/WP_AssetInformation.FilterSpeedSlider` (`self.AssetInformationWidget`)))))
  (bind _returnvalue_3 (- _maltclumpscontent _returnvalue_2))
  (`parent.ReceiveTick` DeltaSeconds)
  (`self.CheckBeerStatus`)
  (if (and (`self.beerNeedsProcessing`) (`self.isProcessing`))
    (set `/Game/IWP/Blueprint/BP_BeerFluid.FiltrationLevel` (+ (`/Game/IWP/Blueprint/BP_BeerFluid.FiltrationLevel` _beerfluid) _returnvalue_2) _beerfluid) ; Calculate the filtering progress
    (bind _output_get (set `self.MaltResiduals` (+ (`self.MaltResiduals`) _returnvalue_2))) ; Increase malt residuals
    (set `self.CloggingLevel` (+ (`self.CloggingLevel`) (* DeltaSeconds (+ (`KismetMathLibrary.SelectFloat` 0.05 0.0 (> _output_get (`self.ResidualsAffectingPumpThreshold`))) (`/Game/IWP/Blueprint/BP_BeerFluid.MaltClumpsContent` (`self.BeerFluid`)) (`KismetMathLibrary.SelectFloat` 0.05 0.0 (> _returnvalue 0.65))) _returnvalue))) ; Increase clogging level based on speed and malt clumps
    (if (> _maltclumpscontent 0.0)
      (set `/Game/IWP/Blueprint/BP_BeerFluid.MaltClumpsContent` (`KismetMathLibrary.SelectFloat` 0.0 _returnvalue_3 (< _returnvalue_3 0.0)) _beerfluid_2) ; Reduce malt clumps and clamp to 0
    )
    (if (>= (`self.CloggingLevel`) 1.0)
      (set `self.isProcessing` false))
    (`self.UpdatePumpStatusText`)
    (if (>= (`/Game/IWP/Blueprint/BP_BeerFluid.FiltrationLevel` (`self.BeerFluid`)) 1.0)
      (set `self.isProcessing` false)
      (`KismetSystemLibrary.PrintString` "Finished filtering")
      (`SceneComponent.SetVisibility` (`self.WP_Transfer_Popup`) true false))
    (else
      (bind _output_get_2 (set `self.IdleTime` (+ DeltaSeconds (`self.IdleTime`)))) ; Increase idle time to determine if residuals start rotting
      (if (and (> _output_get_2 15.0) (> (`self.MaltResiduals`) 0.0))
        (set `self.Contamination` (+ (`self.Contamination`) (* DeltaSeconds 0.1))) ; Increase contamination based on time
      ))))

(event `self.TransferButton`
  (`parent.TransferButton`)
  (`self.TransferBeerFluid` "/Game/IWP/Blueprint/BP_CookingTank.BP_CookingTank_C"))

(fn `CheckBeerStatus`
  (bind _beerfluid (`self.BeerFluid`))
  (`/Engine/EditorBlueprintResources/StandardMacros.IsValid` _beerfluid
    (:`Is Valid`
      (set `self.beerNeedsProcessing` (< (`/Game/IWP/Blueprint/BP_BeerFluid.FiltrationLevel` _beerfluid) 1.0)))
    (:`Is Not Valid`
      (set `self.beerNeedsProcessing` false))))

(fn `CleanBuilding`
  (`parent.CleanBuilding`)
  (set `self.Contamination` 0.0)
  (set `self.MaltResiduals` 0.0)
  (set `self.IdleTime` 0.0))

(fn `CleanPump`
  (if (`KismetSystemLibrary.IsValid` (`self.BeerFluid`))
    (set `self.BeerFluidAmount` (* (`self.BeerFluidAmount`) (`self.PumpCleaningFluidLoss`)))
    (`KismetArrayLibrary.Array_Add` (`/Game/IWP/Blueprint/BP_BeerFluid.FailLog` (`self.BeerFluid`)) "Lost beer by cleaning filter pump while tank is filled"))
  (set `self.CloggingLevel` 0.0))

(fn `UpdatePumpStatusText`
  (bind _filtepumpstatustext (`/Game/IWP/Blueprint/Widgets/WP_AssetInformation.FiltePumpStatusText` (`self.AssetInformationWidget`)))
  (if (>= (`self.CloggingLevel`) 1.0)
    (`TextBlock.SetText` _filtepumpstatustext "Clogged")
    (elif (>= (`self.CloggingLevel`) 0.65)
      (`TextBlock.SetText` _filtepumpstatustext "Hindered")
      (else
        (`TextBlock.SetText` _filtepumpstatustext "Clear")))))

(fn `UserConstructionScript`
  (`parent.UserConstructionScript`))