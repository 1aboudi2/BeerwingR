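; BP_Cube is an actor with a world-space transfer popup, apparently a base for children that transfer beer fluid.
; TransferPopup binds the widget's ready press to TransferButton, caches the popup's location and hides it.
; HidePopup turns off visibility and teleports the widget down by an offset, while ShowPopup restores both.
; TransferButton only prints and hides the popup; a note leaves the TransferBeerFluid call to children.
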(event `Transfer Popup`
  (bind _wp_transfer_popup_2 (`self.WP_Transfer_Popup_2`))
  ;[0.9317 0.04025 1] Transfer Popup (make sure to show popup when the asset is finished)
  (bind _aswp_transfer_popup (cast `/Game/IWP/Blueprint/Widgets/WP_Transfer_Popup` (`WidgetComponent.GetWidget` _wp_transfer_popup_2)))
  (add `/Game/IWP/Blueprint/Widgets/WP_Transfer_Popup.TransferReady_Popup_Pressed` _aswp_transfer_popup (delegate `TransferButton`))
  (set `self.Original Popup Location` (`SceneComponent.K2_GetComponentLocation` _wp_transfer_popup_2))
  (`self.Hide Popup`))

(event `TransferButton`
  ;[0.9317 0.04025 1] Transfer Popup (make sure to show popup when the asset is finished)
  (`KismetSystemLibrary.PrintString` "Transfer button clicked")
  (`self.Hide Popup`))

(event `Hide Popup`
  (bind _wp_transfer_popup_2 (`self.WP_Transfer_Popup_2`))
  (bind (_original_popup_location_x _original_popup_location_y _original_popup_location_z) (`KismetMathLibrary.BreakVector` (`self.Original Popup Location`)))
  ;[0.9317 0.04025 1] Transfer Popup (make sure to show popup when the asset is finished)
  (`SceneComponent.SetVisibility` _wp_transfer_popup_2 false false)
  (`SceneComponent.K2_SetWorldLocation` _wp_transfer_popup_2 (`KismetMathLibrary.MakeVector` _original_popup_location_x _original_popup_location_y (- _original_popup_location_z (`self.Hide Popup Offset`))) false true))

(event `Show Popup`
  (bind _wp_transfer_popup_2 (`self.WP_Transfer_Popup_2`))
  ;[0.9317 0.04025 1] Transfer Popup (make sure to show popup when the asset is finished)
  (`SceneComponent.SetVisibility` _wp_transfer_popup_2 true false)
  (`SceneComponent.K2_SetWorldLocation` _wp_transfer_popup_2 (`self.Original Popup Location`) false true))

(fn `UserConstructionScript`)