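; BP_FakeAsset is an interactive placeholder asset with a cube component that shows its title and description in an information widget.
; On BeginPlay it creates its own WP_AssetInformation widget and adds it to the viewport.
; Ending a touch on the cube or pressing the left mouse button anywhere toggles a Clicked flag.
; Toggling on calls AssetMenu and fills the widget's texts; toggling off only clears the flag.
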(event `self.ReceiveBeginPlay`
  (bind _returnvalue (`|CreateWidget` "/Game/IWP/Blueprint/Widgets/WP_AssetInformation.WP_AssetInformation_C"))
  (bind _output_get (set `self.AssetInformationWidget` _returnvalue))
  (`UserWidget.AddToViewport` _output_get 0))

(event `self.FakeAssetCube.OnInputTouchEnd`
  (params (FingerIndex :type "ETouchIndex Enum" :default "Touch1") (TouchedComponent :type "PrimitiveComponent Object Reference"))
  (bind _assetinformationwidget (`self.AssetInformationWidget`))
  (if (`self.Clicked`) :!label _label
    (set `self.Clicked` false)
    (else
      (set `self.Clicked` true)
      (`/Game/IWP/Blueprint/Widgets/WP_AssetInformation.Asset menu` (`self.AssetInformationWidget`))
      (set `TextBlock.Text` (`self.AssetTitle`) (`/Game/IWP/Blueprint/Widgets/WP_AssetInformation.AssetTitle` _assetinformationwidget))
      (set `TextBlock.Text` (`self.AssetInformation`) (`/Game/IWP/Blueprint/Widgets/WP_AssetInformation.AssetInformation` _assetinformationwidget)))))

(event `Key|LeftMouseButton`
  (params (Key :type "Key Structure"))
  (:`Pressed`
    (`KismetSystemLibrary.PrintString` "click")
    (goto _label)))

(fn `UserConstructionScript`)