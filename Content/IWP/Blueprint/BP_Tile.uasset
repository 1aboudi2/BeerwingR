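; BP_Tile is a grid tile actor that knows its row, column and array position and records when it becomes occupied.
; InitializeTile attaches the tile to its owner, then offsets it by column and row using twice the Tile component's box extent, so spacing follows its bounds.
; Any actor overlap sets Occupied and prints the array position; nothing here clears the flag, and the parent-actor validity check leads nowhere.
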(event `self.ReceiveActorBeginOverlap`
  (params (OtherActor :type "Actor Object Reference"))
  (set `self.Occupied` true)
  (`KismetSystemLibrary.PrintString` (`KismetStringLibrary.Conv_IntToString` (`self.PosInArray`)))
  (`/Engine/EditorBlueprintResources/StandardMacros.IsValid` (`self.GetAttachParentActor`)))

(fn `InitializeTile`
  (bind _returnvalue (`self.GetOwner`))
  (`/Engine/EditorBlueprintResources/StandardMacros.IsValid` _returnvalue
    (:`Is Valid`
      (`self.K2_AttachToActor` _returnvalue "None" "SnapToTarget" "SnapToTarget" "KeepRelative" false)
      (`self.K2_SetActorRelativeLocation` (`KismetMathLibrary.MakeVector` (* (.x (`.BoxExtent` (`KismetSystemLibrary.GetComponentBounds` (`self.Tile`)))) (`self.Column`) 2.0) (* (.y (`.BoxExtent` (`KismetSystemLibrary.GetComponentBounds` (`self.Tile`)))) (`self.Row`) 2.0))))))

(fn `UserConstructionScript`)