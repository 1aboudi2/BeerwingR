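; BP_BeerTesters is an NPC beer taster that reacts when the player presses a beer-ready popup.
; It rebinds to every WP_Popup each Tick, and a press rolls a random quality that picks a happy or sad emoticon.
; The emoticon shows briefly, then a WP_BeerFeedback widget lists BeerFluid's FailLog, which does not affect the random verdict.
; On BeginPlay, its NPC text turns once relative to the player's rotation.
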(event `self.ReceiveBeginPlay`
  (bind (_returnvalue_roll _returnvalue_pitch _returnvalue_yaw) (`KismetMathLibrary.BreakRotator` (`self.K2_GetActorRotation` (`GameplayStatics.GetPlayerPawn` 0))))
  (`|ExecutionSequence`
    (:`then_0`
      (bind _aswp_emoticon (cast `/Game/IWP/Blueprint/Widgets/WP_Emoticon` (`WidgetComponent.GetWidget` (`self.Emoticon`)))
        (:`then`
          (set `self.EmoticonWidget` _aswp_emoticon)
          (`SceneComponent.SetVisibility` (`self.Emoticon`) false false))
        (:`CastFailed`
          (`KismetSystemLibrary.PrintString` "no emoticon" true true (struct :`R` 1.0 :`G` 0.870887 :`A` 1.0) 5.0))))
    (:`then_1`
      (`self.BindEventToPopup`))
    (:`then_2`
      (`SceneComponent.K2_SetWorldRotation` (`self.NPC text`) (`KismetMathLibrary.MakeRotator` _returnvalue_roll _returnvalue_pitch (+ _returnvalue_yaw 180.0)) false false))
    (:`then_3`
      (set `self.isBeerReceiver` true))))

(event `Emotion Choosinator`
  (params (`Reaction ID` :type Integer))
  (bind _emoticonwidget (`self.EmoticonWidget`))
  (bind _emoticonwidget_2 (`self.EmoticonWidget`))
  ;[0 0.3047 1] Emotion Choosinator
  (if (== `Reaction ID` 0)
    (`Widget.SetVisibility` (`/Game/IWP/Blueprint/Widgets/WP_Emoticon.Happy` _emoticonwidget_2) "Hidden")
    (`Widget.SetVisibility` (`/Game/IWP/Blueprint/Widgets/WP_Emoticon.Sad` _emoticonwidget_2) "Visible")
    (else
      (`Widget.SetVisibility` (`/Game/IWP/Blueprint/Widgets/WP_Emoticon.Happy` _emoticonwidget) "Visible")
      (`Widget.SetVisibility` (`/Game/IWP/Blueprint/Widgets/WP_Emoticon.Sad` _emoticonwidget) "Hidden"))))

(event `self.ReceiveTick`
  (params (DeltaSeconds :type "Float (single-precision)"))
  (`self.BindEventToPopup`))

(event `Emotion Showinator`
  ;[0 1 0.8336] Emotion Showinator
  (`SceneComponent.SetVisibility` (`self.Emoticon`) true false)
  (`KismetSystemLibrary.Delay` 2.0)
  (`SceneComponent.SetVisibility` (`self.Emoticon`) false false)
  (`self.FeedbackLog`))

(event `BindEventToPopup`
  (bind _foundwidgets (`WidgetBlueprintLibrary.GetAllWidgetsOfClass` "/Game/IWP/Blueprint/Widgets/WP_Popup.WP_Popup_C" false))
  (for (_array_element _array_index) _foundwidgets
    (bind _output_get (set `self.currentPopup` _array_element))
    (`/Engine/EditorBlueprintResources/StandardMacros.IsValid` _output_get
      (:`Is Valid`
        (add `/Game/IWP/Blueprint/Widgets/WP_Popup.BeerReady_Popup_Pressed` _output_get (delegate `Beer Emoticon Popup`)))
      (:`Is Not Valid`
        (`KismetSystemLibrary.PrintString` "not detected popup" true true (struct :`R` 1.0 :`B` 0.19292 :`A` 1.0) 10.0)))))

(event `Beer Emoticon Popup`
  ;[1 0.0172 0] Event Emoticon Popup
  (bind _beerquality (`self.BeerQualityRandomizer`))
  (bind _reactionid (`self.Quality Checker` _beerquality))
  (`self.Emotion Choosinator` _reactionid)
  (`self.Emotion Showinator`)
  (`KismetSystemLibrary.PrintString` (`KismetStringLibrary.Conv_IntToString` _reactionid)))

(event `FeedbackLog`
  (bind _returnvalue (`|CreateWidget` "/Game/IWP/Blueprint/Widgets/WP_BeerFeedback.WP_BeerFeedback_C"))
  (bind _output_get (set `self.BeerFeedback` _returnvalue))
  (`UserWidget.AddToViewport` _output_get 0)
  (`TextBlock.SetText` (`/Game/IWP/Blueprint/Widgets/WP_BeerFeedback.Fails` (`self.BeerFeedback`)) (`KismetTextLibrary.Conv_StringToText` (`KismetStringLibrary.JoinStringArray` (`/Game/IWP/Blueprint/BP_BeerFluid.FailLog` (`self.BeerFluid`)) ","))))

(fn `BeerQualityRandomizer`
  (returns (BeerQuality :type Integer))
  (bind _output_get (set `self.Beer Quality` (`KismetMathLibrary.RandomIntegerInRange` 1 10)))
  (return _output_get))

(fn `Quality Checker`
  (params (`Beer Quality Input` :type Integer))
  (returns (ReactionID :type Integer))
  (if (<= `Beer Quality Input` 5)
    (return 0)
    (else
      (return 1))))

(fn `UserConstructionScript`)