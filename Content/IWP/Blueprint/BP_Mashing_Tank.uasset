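; Mashing Tank building for a brewing process, a beer receiver that mixes water and malt and transfers the fluid to the filtration building.
; Shows its info-widget controls; Add Water creates or increments BeerFluid.
; Start/Stop activates the Spin component for SpinningTime while flagged as mashing.
; Tick mirrors pH and blade-speed sliders to text and feeds blade speed into MALTA for malt logic, which is still mostly debug prints.
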(event `self.ReceiveBeginPlay`
  (`parent.ReceiveBeginPlay`)
  (set `self.isBeerReceiver` true)
  (set `self.AssetTitle` "Mashing Tank")
  (set `self.AssetInformation` "Mix Water and grinded Malt to extract the flavour")
  (`Widget.SetVisibility` (`/Game/IWP/Blueprint/Widgets/WP_AssetInformation.Start-Stop_ButtonContainer` (`self.AssetInformationWidget`)) "SelfHitTestInvisible")
  (`Widget.SetVisibility` (`/Game/IWP/Blueprint/Widgets/WP_AssetInformation.TransferContainer` (`self.AssetInformationWidget`)) "SelfHitTestInvisible")
  (`Widget.SetVisibility` (`/Game/IWP/Blueprint/Widgets/WP_AssetInformation.BladeSpeed` (`self.AssetInformationWidget`)) "SelfHitTestInvisible")
  (`Widget.SetVisibility` (`/Game/IWP/Blueprint/Widgets/WP_AssetInformation.AddWater` (`self.AssetInformationWidget`)) "SelfHitTestInvisible")
  (`Widget.SetVisibility` (`/Game/IWP/Blueprint/Widgets/WP_AssetInformation.AddMalt` (`self.AssetInformationWidget`)) "SelfHitTestInvisible") ; you can combine all the set visibilities into 1
  (add `/Game/IWP/Blueprint/Widgets/WP_AssetInformation.AddWaterFluidDispatcher` (`self.AssetInformationWidget`) (delegate `AddWaterButton`)))

(event `AddWaterButton`
  (`KismetSystemLibrary.PrintString` "waterB clicked")
  (`self.addWaterF`))

(event `self.ReceiveTick`
  (params (DeltaSeconds :type "Float (single-precision)"))
  (bind _assetinformationwidget (`self.AssetInformationWidget`))
  (bind _returnvalue (`KismetMathLibrary.Round64` (`Slider.GetValue` (`/Game/IWP/Blueprint/Widgets/WP_AssetInformation.BladeSpeedSlider` _assetinformationwidget))))
  (`parent.ReceiveTick` DeltaSeconds)
  (`TextBlock.SetText` (`/Game/IWP/Blueprint/Widgets/WP_AssetInformation.CurrentpH` _assetinformationwidget) (`KismetTextLibrary.Conv_Int64ToText` (`KismetMathLibrary.Round64` (`Slider.GetValue` (`/Game/IWP/Blueprint/Widgets/WP_AssetInformation.pHSlider` _assetinformationwidget))))) ; Set the pH text to the slider's value
  (`TextBlock.SetText` (`/Game/IWP/Blueprint/Widgets/WP_AssetInformation.CurrentBladeSpeed` _assetinformationwidget) (`KismetTextLibrary.Conv_Int64ToText` _returnvalue)) ; Set the Blade Speed text to the slider's value
  (set `self.MALT_A` _returnvalue)
  (`self.addmalt_F` DeltaSeconds))

(event `self.StartStopButton`
  (`parent.StartStopButton`)
  (`self.startMashing`))

(event `self.TransferButton`
  (`parent.TransferButton`)
  (`self.TransferBeerFluid` "/Game/IWP/Blueprint/BP_Filtration_Building.BP_Filtration_Building_C"))

(event `startMashing`
  ;[1 1 1] settiing up the spinning top + start mash function
  (`KismetSystemLibrary.PrintString` "mashing on")
  (set `self.IsMashing` true)
  (`self.spinningTop`))

(event `spinningTop`
  ;[1 1 1] settiing up the spinning top + start mash function
  (`KismetSystemLibrary.PrintString` "startingspinning")
  (`ActorComponent.SetActive` (`self.spin`) true false)
  (`KismetSystemLibrary.Delay` (`self.spinningTime`))
  (`ActorComponent.SetActive` (`self.spin`) false false)
  (`KismetSystemLibrary.PrintString` "spinningdone")
  (set `self.IsMashing` false))

(fn `addmalt_F`
  (params (deltatime :type "Float (double-precision)"))
  (`/Engine/EditorBlueprintResources/StandardMacros.IsValid` (`self.BeerFluid`)
    (:`Is Not Valid`
      (if (> (`self.MALT_A`) 0)
        (if (`self.IsMashing`)
          (`KismetSystemLibrary.PrintString` "do calc")
          (set `self.Previus_MALT_A` (`KismetMathLibrary.Conv_Int64ToInt` (`self.MALT_A`)))
          (else
            (`KismetSystemLibrary.PrintString` "clumpsing")))))))

(fn `addWaterF`
  (bind _beerfluidamount (`self.BeerFluidAmount`))
  (`/Engine/EditorBlueprintResources/StandardMacros.IsValid` (`self.BeerFluid`)
    (:`Is Valid`
      (`/Engine/EditorBlueprintResources/StandardMacros.IncrementFloat` _beerfluidamount
        (:`  `
          (`KismetSystemLibrary.PrintString` (`KismetStringLibrary.Conv_DoubleToString` _beerfluidamount)))))
    (:`Is Not Valid`
      (bind _returnvalue (`|GenericCreateObject` "/Game/IWP/Blueprint/BP_BeerFluid.BP_BeerFluid_C"))
      (set `self.BeerFluid` _returnvalue)
      (set `self.BeerFluidAmount` 1.0)
      (`KismetSystemLibrary.PrintString` "wateradded"))))

(fn `clearWaterFluid`
  (set `self.WaterFluid` null)
  (set `self.Water Fluid Amount` 0.0))

(fn `UserConstructionScript`
  (`parent.UserConstructionScript`))