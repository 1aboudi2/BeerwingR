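; Fermentation tank building for a brewing game that turns received beer fluid into fermented beer using player-added yeast.
; Tick eases fluid temperature toward the widget slider, kills overheated yeast, and advances fermentation while building pressure that explodes the tank at its limit.
; Fluid left without yeast spoils, and an uncleaned empty tank accumulates contamination that passes to the next batch.
; Widget dispatchers drive yeast and pressure-release input, though release only sets a flag here.
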(event `self.ReceiveBeginPlay`
  (bind _assetinformationwidget (`self.AssetInformationWidget`))
  (bind _assetinformationwidget_2 (`self.AssetInformationWidget`))
  (`parent.ReceiveBeginPlay`)
  (set `self.isBeerReceiver` true)
  (set `self.AssetTitle` "Fermentation Tank")
  (set `self.AssetInformation` "Using yeast to ferment the wort")
  (`Widget.SetVisibility` (`/Game/IWP/Blueprint/Widgets/WP_AssetInformation.Temperature` _assetinformationwidget) "SelfHitTestInvisible")
  (`Widget.SetVisibility` (`/Game/IWP/Blueprint/Widgets/WP_AssetInformation.TransferContainer` _assetinformationwidget) "SelfHitTestInvisible")
  (`Widget.SetVisibility` (`/Game/IWP/Blueprint/Widgets/WP_AssetInformation.PressureInformationContainer` _assetinformationwidget) "SelfHitTestInvisible")
  (`Widget.SetVisibility` (`/Game/IWP/Blueprint/Widgets/WP_AssetInformation.AddYeastContainer` _assetinformationwidget) "SelfHitTestInvisible")
  (`|ExecutionSequence`
    (:`then_0`
      (add `/Game/IWP/Blueprint/Widgets/WP_AssetInformation.AddYeastButtonDispatcher` _assetinformationwidget_2 (delegate `YeastButtonClicked`)))
    (:`then_1`
      (add `/Game/IWP/Blueprint/Widgets/WP_AssetInformation.ReleasePressureClickedDispatcher` _assetinformationwidget_2 (delegate `ReleasePressureButtonClicked`)))
    (:`then_2`
      (add `/Game/IWP/Blueprint/Widgets/WP_AssetInformation.ReleasePressurePressedDispatcher` _assetinformationwidget_2 (delegate `ReleasePressureButtonPressed`)))
    (:`then_3`
      (add `/Game/IWP/Blueprint/Widgets/WP_AssetInformation.ReleasePressureReleasedDispatcher` _assetinformationwidget_2 (delegate `ReleasePressureButtonReleased`)))))

(event `YeastButtonClicked`
  (bind _beerfluid (`self.BeerFluid`))
  (`/Engine/EditorBlueprintResources/StandardMacros.IsValid` _beerfluid
    (:`Is Valid`
      (`/Engine/EditorBlueprintResources/StandardMacros.IncrementFloat` (`/Game/IWP/Blueprint/BP_BeerFluid.YeastStrength` _beerfluid)
        (:`  `
          (set `self.IdleTimeWithoutYeast` 0.0)
          (set `self.Pressure` 0.1))))))

(event `self.TransferButton`
  (`parent.TransferButton`)
  (`self.TransferBeerFluid` "BP_Fermentation_Building_C"))

(event `ReleasePressureButtonClicked`)

(event `ReleasePressureButtonPressed`
  (set `self.isReleasingPressure` true))

(event `ReleasePressureButtonReleased`
  (set `self.isReleasingPressure` false))

(event `self.ReceiveTick`
  (params (DeltaSeconds :type "Float (single-precision)"))
  (bind (_returnvalue_x _returnvalue_y) (`KismetMathLibrary.BreakVector` (`self.K2_GetActorLocation`)))
  (bind _beerfluid (`self.BeerFluid`))
  (bind _beerfluid_2 (`self.BeerFluid`))
  (bind _idletimewithoutyeast (`self.IdleTimeWithoutYeast`))
  (bind _idletimewithoutyeastthreshold (`self.IdleTimeWithoutYeastThreshold`))
  (bind _beerfluid_3 (`self.BeerFluid`))
  (bind _beerfluid_4 (`self.BeerFluid`))
  (bind _returnvalue (+ _idletimewithoutyeast DeltaSeconds))
  (bind _returnvalue_2 (>= _returnvalue _idletimewithoutyeastthreshold))
  (bind _returnvalue_3 (+ (`/Game/IWP/Blueprint/BP_BeerFluid.FermentationLevel` _beerfluid) (* (`self.FermentationMultiplier`) (`KismetMathLibrary.Sqrt` (`/Game/IWP/Blueprint/BP_BeerFluid.YeastStrength` _beerfluid)) DeltaSeconds)))
  (if (`self.isDead`)
    (bind _returnvalue_4 (`GameplayStatics.GetActorOfClass` "/Game/IWP/Blueprint/BP_GridSystem.BP_GridSystem_C"))
    (bind _index (`/Game/IWP/Blueprint/BP_GridSystem.GetIndexFromPos` _returnvalue_4 _returnvalue_x _returnvalue_y))
    (`KismetArrayLibrary.Array_Set` (`/Game/IWP/Blueprint/BP_GridSystem.isTileOccupied` _returnvalue_4) _index)
    (`self.K2_DestroyActor`)
    (else
      (`parent.ReceiveTick` DeltaSeconds)
      (`/Engine/EditorBlueprintResources/StandardMacros.IsValid` _beerfluid_2
        (:`Is Valid`
          (bind _resultvalue (`self.CalculateMovingValue` (`/Game/IWP/Blueprint/BP_BeerFluid.Temperature` _beerfluid_2) (`Slider.GetValue` (`/Game/IWP/Blueprint/Widgets/WP_AssetInformation.TempSlider` (`self.AssetInformationWidget`))) DeltaSeconds (`self.TemperatureChangeRate`)))
          (bind _output_get (set `/Game/IWP/Blueprint/BP_BeerFluid.Temperature` _resultvalue (`self.BeerFluid`)))
          (`|ExecutionSequence`
            (:`then_0`
              ;[1 1 1] Yeast dying
              (if (>= _output_get (`self.YeastDeathThreashold`))
                (set `/Game/IWP/Blueprint/BP_BeerFluid.YeastStrength` 0.0 _beerfluid_3)
                (`KismetArrayLibrary.Array_Add` (`/Game/IWP/Blueprint/BP_BeerFluid.FailLog` _beerfluid_3) "Yeast died due to high fluid temperature")))
            (:`then_1`
              ;[1 1 1] Fermentation
              (if (not (`self.isDoneFermenting`))
                (if (> (`/Game/IWP/Blueprint/BP_BeerFluid.YeastStrength` (`self.BeerFluid`)) 0.0)
                  (bind _output_get_2 (set `/Game/IWP/Blueprint/BP_BeerFluid.FermentationLevel` (`KismetMathLibrary.SelectFloat` 1.0 _returnvalue_3 (>= _returnvalue_3 1.0)) _beerfluid))
                  (if (>= _output_get_2 1.0)
                    (set `self.isDoneFermenting` true)
                    (else
                      ;[1 1 1] Pressure
                      (bind _output_get_3 (set `self.Pressure` (+ (`self.Pressure`) (/ (* (`self.FermentationMultiplier`) (`/Game/IWP/Blueprint/BP_BeerFluid.YeastStrength` (`self.BeerFluid`)) DeltaSeconds) 2.5))))
                      (if (>= _output_get_3 1.0)
                        (`GameplayStatics.SpawnEmitterAtLocation` "/Game/StarterContent/Particles/P_Explosion.P_Explosion" (`self.K2_GetActorLocation`))
                        (set `self.isDead` true))))
                  (else
                    ;[1 1 1] Idle without yeast and therefore spoiling
                    (if (< (`/Game/IWP/Blueprint/BP_BeerFluid.Temperature` (`self.BeerFluid`)) (`self.YeastDeathThreashold`))
                      (if (and _returnvalue_2 (< _idletimewithoutyeast _idletimewithoutyeastthreshold))
                        (`KismetArrayLibrary.Array_Add` (`/Game/IWP/Blueprint/BP_BeerFluid.FailLog` (`self.BeerFluid`)) "Fluid started spoiling by idling too long in the fermentation tank"))
                      (set `self.IdleTimeWithoutYeast` _returnvalue)
                      (if _returnvalue_2
                        (set `/Game/IWP/Blueprint/BP_BeerFluid.Contamination` (+ (* DeltaSeconds 0.1) (`/Game/IWP/Blueprint/BP_BeerFluid.Contamination` _beerfluid_4)) _beerfluid_4)))))))))
        (:`Is Not Valid`
          (if (`self.hasResiduals`)
            (bind _output_get_4 (set `self.IdleTimeEmpty` (+ DeltaSeconds (`self.IdleTimeEmpty`))))
            (if (>= _output_get_4 15.0)
              (set `self.Contamination` (+ (* DeltaSeconds 0.1) (`self.Contamination`))))))))))

(fn `CalculateMovingValue`
  (params (CurrentValue :type "Float (double-precision)") (TargetValue :type "Float (double-precision)") (DeltaTime :type "Float (double-precision)") (ChangeRate :type "Float (double-precision)"))
  (returns (ResultValue :type "Float (double-precision)"))
  (bind _returnvalue (* DeltaTime ChangeRate))
  (bind _returnvalue_2 (- CurrentValue _returnvalue))
  (bind _returnvalue_3 (+ CurrentValue _returnvalue))
  (if (== CurrentValue TargetValue)
    (return CurrentValue)
    (else
      (if (> CurrentValue TargetValue)
        (if (< _returnvalue_2 TargetValue)
          _
          (else
            (return _returnvalue_2)))
        (elif (> _returnvalue_3 TargetValue)
          _
          (else
            (return _returnvalue_3))))
      (return TargetValue))))

(fn `CleanBuilding`
  (`parent.CleanBuilding`)
  (set `self.Contamination` 0.0)
  (set `self.hasResiduals` false)
  (set `self.IdleTimeEmpty` 0.0))

(fn `ClearBeerFluid`
  (`parent.ClearBeerFluid`)
  (set `self.Pressure` (`self.RestingPressure`))
  (set `self.hasResiduals` true)
  (set `self.IdleTimeWithoutYeast` 0.0)
  (set `self.isDoneFermenting` false))

(fn `ReceiveBeerFluid`
  (params (IncomingBeerFluid :type "/Game/IWP/Blueprint/BP_BeerFluid Object Reference") (FluidAmount :type "Float (double-precision)"))
  (returns (Accpeted :type Boolean))
  (bind _beerfluid (`self.BeerFluid`))
  (bind _accpeted (`parent.ReceiveBeerFluid` IncomingBeerFluid FluidAmount))
  (if (and _accpeted (> (`self.Contamination`) 0.0))
    (`KismetArrayLibrary.Array_Add` (`/Game/IWP/Blueprint/BP_BeerFluid.FailLog` _beerfluid) "Contaminated by using an unclean fermentation tank")
    (set `/Game/IWP/Blueprint/BP_BeerFluid.Contamination` (+ (`/Game/IWP/Blueprint/BP_BeerFluid.Contamination` _beerfluid) (`self.Contamination`)) _beerfluid))
  (return _accpeted))

(fn `UserConstructionScript`
  (`parent.UserConstructionScript`))