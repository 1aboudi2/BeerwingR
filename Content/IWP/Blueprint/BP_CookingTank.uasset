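; Cooking Tank building for the brewing game, which heats received beer fluid and targets the fermentation building for transfer.
; When switched on, Tick moves fluid temperature toward the widget slider, and a Timeline raises CookingLevel in the boiling range.
; Prolonged boiling after the Timeline finishes drains fluid until the tank explodes and frees its grid tile.
; An empty tank builds up mold contamination over time, which passes to the next batch unless cleaned.
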(event `self.ReceiveBeginPlay`
  (`parent.ReceiveBeginPlay`)
  (set `self.Target Class` "/Game/IWP/Blueprint/BP_Fermentation_Building.BP_Fermentation_Building_C")
  (set `self.isBeerReceiver` true)
  (set `self.AssetTitle` "Cooking Tank")
  (set `self.AssetInformation` "")
  (`Widget.SetVisibility` (`/Game/IWP/Blueprint/Widgets/WP_AssetInformation.Temperature` (`self.AssetInformationWidget`)) "SelfHitTestInvisible")
  (`Widget.SetVisibility` (`/Game/IWP/Blueprint/Widgets/WP_AssetInformation.Start-Stop_ButtonContainer` (`self.AssetInformationWidget`)) "SelfHitTestInvisible")
  (`Widget.SetVisibility` (`/Game/IWP/Blueprint/Widgets/WP_AssetInformation.AddHops` (`self.AssetInformationWidget`)) "SelfHitTestInvisible")
  (`Widget.SetVisibility` (`/Game/IWP/Blueprint/Widgets/WP_AssetInformation.TransferContainer` (`self.AssetInformationWidget`)) "SelfHitTestInvisible")
  (add `/Game/IWP/Blueprint/Widgets/WP_AssetInformation.StartStopButtonDispatcher` (`self.AssetInformationWidget`) (delegate `Cooking`)))

(event `Cooking`
  (if (`self.On/Off`)
    (set `self.On/Off` false)
    (`SceneComponent.SetVisibility` (`self.P_Steam_Lit`) false false)
    (else
      (set `self.On/Off` true)
      (`SceneComponent.SetVisibility` (`self.P_Steam_Lit`) true false))))

(event `self.TransferButton`
  (`parent.TransferButton`)
  (goto _label :!via `Reset`))

(event `self.ReceiveTick`
  (params (DeltaSeconds :type "Float (single-precision)"))
  (bind (_returnvalue_x _returnvalue_y) (`KismetMathLibrary.BreakVector` (`self.K2_GetActorLocation`)))
  (bind _beerfluid (`self.BeerFluid`))
  (bind _returnvalue (+ DeltaSeconds (`self.overboilingTime`)))
  (`parent.ReceiveTick` DeltaSeconds)
  (if (`self.isDead`)
    (bind _returnvalue_2 (`GameplayStatics.GetActorOfClass` "/Game/IWP/Blueprint/BP_GridSystem.BP_GridSystem_C"))
    (bind _index (`/Game/IWP/Blueprint/BP_GridSystem.GetIndexFromPos` _returnvalue_2 _returnvalue_x _returnvalue_y))
    (`KismetArrayLibrary.Array_Set` (`/Game/IWP/Blueprint/BP_GridSystem.isTileOccupied` _returnvalue_2) _index)
    (`self.K2_DestroyActor`)
    (else
      (`/Engine/EditorBlueprintResources/StandardMacros.IsValid` (`self.BeerFluid`)
        (:`Is Valid`
          (if (`self.On/Off`)
            (`/Engine/EditorBlueprintResources/StandardMacros.IsValid` (`self.BeerFluid`)
              (:`Is Valid`
                (bind _resultvalue (`self.CalculateMovingValueTowardsTarget` (`/Game/IWP/Blueprint/BP_BeerFluid.Temperature` (`self.BeerFluid`)) (`Slider.GetValue` (`/Game/IWP/Blueprint/Widgets/WP_AssetInformation.TempSlider` (`self.AssetInformationWidget`))) DeltaSeconds (`self.TempChangeRate`)))
                (bind _output_get (set `/Game/IWP/Blueprint/BP_BeerFluid.Temperature` _resultvalue (`self.BeerFluid`)))
                (`TextBlock.SetText` (`/Game/IWP/Blueprint/Widgets/WP_AssetInformation.CurrentTemp` (`self.AssetInformationWidget`)) (`KismetTextLibrary.Conv_DoubleToText` _output_get "HalfToEven" false true 1 324 0 0))
                (if (and (>= _output_get 100.0) (<= _output_get 120.0))
                  (`Timeline|Timeline`
                    (:`Update`
                      (set `/Game/IWP/Blueprint/BP_BeerFluid.CookingLevel` (+ (* DeltaSeconds 0.2) (`/Game/IWP/Blueprint/BP_BeerFluid.CookingLevel` _beerfluid)) _beerfluid))
                    (:`Finished`
                      (`|ExecutionSequence`
                        (:`then_0`
                          (`/Engine/EditorBlueprintResources/StandardMacros.DoOnce` false :!label _label
                            (:`Completed`
                              (`self.Show Popup`))))
                        (:`then_1`
                          (if (>= _returnvalue 10.0)
                            (if (< (`self.overboilingTime`) 10.0)
                              (`KismetArrayLibrary.Array_Add` (`/Game/IWP/Blueprint/BP_BeerFluid.FailLog` (`self.BeerFluid`)) "Losing fluid due to overboiling"))
                            (set `self.overboilingTime` _returnvalue)
                            (bind _output_get_2 (set `self.BeerFluidAmount` (- (`self.BeerFluidAmount`) (* DeltaSeconds 0.05))))
                            (if (<= _output_get_2 0.0)
                              (set `self.isDead` true)
                              (`GameplayStatics.SpawnEmitterAtLocation` "/Game/StarterContent/Particles/P_Explosion.P_Explosion" (`self.K2_GetActorLocation`)))
                            (else
                              (set `self.overboilingTime` _returnvalue)))))))))
              (:`Is Not Valid`
                (if (>= (`Slider.GetValue` (`/Game/IWP/Blueprint/Widgets/WP_AssetInformation.TempSlider` (`self.AssetInformationWidget`))) 69.0)
                  (set `self.isDead` true)
                  (`GameplayStatics.SpawnEmitterAtLocation` "/Game/StarterContent/Particles/P_Explosion.P_Explosion" (`self.K2_GetActorLocation`)))))))
        (:`Is Not Valid`
          (bind _output_get_3 (set `self.moldingTime` (+ (`self.moldingTime`) DeltaSeconds)))
          (if (>= _output_get_3 15.0)
            (set `self.Contamination` (+ (`self.Contamination`) (* DeltaSeconds 0.02)))))))))

(fn `CleanBuilding`
  (`parent.CleanBuilding`)
  (set `self.hasResiduals` false)
  (set `self.overboilingTime` 0.0)
  (set `self.On/Off` false)
  (`SceneComponent.SetVisibility` (`self.P_Steam_Lit`) false false)
  (set `self.moldingTime` 0.0)
  (set `self.Contamination` 0.0))

(fn `ClearBeerFluid`
  (`parent.ClearBeerFluid`)
  (set `self.On/Off` false)
  (`TimelineComponent.SetPlaybackPosition` (`self.Timeline`) 0.0 false false)
  (`SceneComponent.SetVisibility` (`self.P_Steam_Lit`) false false)
  (set `self.overboilingTime` 0.0)
  (set `self.hasResiduals` true)
  (set `self.moldingTime` 0.0))

(fn `ReceiveBeerFluid`
  (params (IncomingBeerFluid :type "/Game/IWP/Blueprint/BP_BeerFluid Object Reference") (FluidAmount :type "Float (double-precision)"))
  (returns (Accpeted :type Boolean))
  (bind _beerfluid (`self.BeerFluid`))
  (bind _accpeted (`parent.ReceiveBeerFluid` IncomingBeerFluid FluidAmount))
  (if _accpeted
    (if (> (`self.Contamination`) 0.0)
      (`KismetArrayLibrary.Array_Add` (`/Game/IWP/Blueprint/BP_BeerFluid.FailLog` _beerfluid) "Increased contamination by using uncleaned cooking tank")
      (set `/Game/IWP/Blueprint/BP_BeerFluid.Contamination` (+ (`/Game/IWP/Blueprint/BP_BeerFluid.Contamination` _beerfluid) (`self.Contamination`)) _beerfluid))
    (return _accpeted)
    (else
      (return _accpeted))))

(fn `UserConstructionScript`
  (`parent.UserConstructionScript`))