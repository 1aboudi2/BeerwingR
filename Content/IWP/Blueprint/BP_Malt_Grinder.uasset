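; BP_Malt_Grinder is a malt grinder asset that supplies its own title and description to an inherited information widget.
; On BeginPlay it runs the parent logic, sets the title and info text, then hides the widget's Temperature and PH fields.
; It adds no grinding logic: overlap and tick events are disabled stubs, and the construction script only calls the parent.
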(event `self.ReceiveBeginPlay`
  (bind _assetinformationwidget (`self.AssetInformationWidget`))
  (`parent.ReceiveBeginPlay`)
  (set `self.AssetTitle` "MaltGrider1")
  (set `self.AssetInformation` "Ready to gride soeme beans?!")
  (`Widget.SetVisibility` (`/Game/IWP/Blueprint/Widgets/WP_AssetInformation.Temperature` _assetinformationwidget) "Hidden")
  (`Widget.SetVisibility` (`/Game/IWP/Blueprint/Widgets/WP_AssetInformation.pH` _assetinformationwidget) "Hidden"))

(fn `UserConstructionScript`
  (`parent.UserConstructionScript`))