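; Touch-driven camera actor with a spring arm that pans in world space by one-finger drag, and adds an Enhanced Input mapping context and main UI widget on BeginPlay.
; Tick normalizes the touch delta into a direction scaled by sensitivity, pausing while the zoom action is active.
; Pinch zoom is unfinished: IA_CameraC sets arm length from a stored value, while the distance-based clamp calculation is left unconnected.
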(event Input|EnhancedActionEvents|EnhancedInputActionIA_CameraC
  (params (ActionValue :type Boolean) (ElapsedSeconds :type Float%20%28double-precision%29) (TriggeredSeconds :type Float%20%28double-precision%29) (InputAction :type Input%20Action%20Object%20Reference :default "/Game/IWP/Input/IA_CameraC.IA_CameraC"))
  ;[1 1 1] Event Begin
  (:Triggered
    (Variables|Default|SetIsZooma true)
    (Variables|/Script/Engine.SpringArmComponent|SetTargetArmLength (Variables|Default|GetSpringArm) (stale _touch_distance))
    (Development|PrintString "double touch"))
  (:Canceled
    (Variables|Default|SetIsZooma false)))

(event EventTick
  (params (DeltaSeconds :type Float%20%28single-precision%29))
  (bind _returnvalue (Game|GetPlayerController 0))
  (bind (_locationx _locationy _biscurrentlypressed) (Class|PlayerController|GetInputTouchState _returnvalue "Touch1"))
  (if (Variables|Default|GetIsZooma)
    (Development|PrintString "ZOOMA!")
    (elif _biscurrentlypressed
      (Variables|Default|SetNew%20Touch%20Location (Math|Vector2D|MakeVector2D _locationx _locationy))
      (Transformation|AddActorWorldOffset (* (Math|Rotator|GetRotationXVector (Math|Conversions|RotationFromXVector (Math|Vector|MakeVector (.y (- (Variables|Default|GetNew%20Touch%20Location) (Variables|Default|GetPrevius%20Touch%20Location))) (* (.x (- (Variables|Default|GetNew%20Touch%20Location) (Variables|Default|GetPrevius%20Touch%20Location))) -1.0) 0.0))) (Variables|Default|GetsensitivityMove)))
      (Variables|Default|SetPrevius%20Touch%20Location (Variables|Default|GetNew%20Touch%20Location)))))

(event EventBeginPlay
  ;[1 1 1] Event Begin
  (bind _asplayer_controller (Utilities|Casting|CastToPlayerController (Game|GetPlayerController 0)))
  ;;[0.05098 0.05098 0.05098] Add Mapping Context
  (Utilities|IsValid (PlayerController|LocalPlayerSubsystems|GetEnhancedInputLocalPlayerSubsystem _asplayer_controller)
    (:Is%20Valid
      (Input|AddMappingContext (PlayerController|LocalPlayerSubsystems|GetEnhancedInputLocalPlayerSubsystem _asplayer_controller) 0 0 "(bIgnoreAllPressedKeysUntilRelease=True,bForceImmediately=False,bNotifyUserSettings=False)")
      (bind _returnvalue (Game|ConstructObjectfromClass (Game|GetPlayerCharacter 0) "/Game/IWP/Blueprint/Widgets/WP_MainUI.WP_MainUI_C"))
      (UserInterface|Viewport|AddtoViewport _returnvalue 0))
    (:Is%20Not%20Valid
      (Development|PrintString "no hello"))))

(event Input|ActionEvents|InputActionDragTouch
  (params (Key :type Key%20Structure :default "None"))
  (bind _returnvalue (Game|GetPlayerController 0))
  (bind (_locationx _locationy) (Class|PlayerController|GetInputTouchState _returnvalue "Touch1"))
  (:Pressed
    (Variables|Default|SetPrevius%20Touch%20Location (Math|Vector2D|MakeVector2D _locationx _locationy))))

(fn ConstructionScript)

(fn GetTouchDistance
  (bind _returnvalue (Game|GetPlayerController 0))
  (bind (_locationx _locationy) (Class|PlayerController|GetInputTouchState _returnvalue "Touch2"))
  (bind (_locationx_2 _locationy_2) (Class|PlayerController|GetInputTouchState _returnvalue "Touch1"))
  (bind (_locationx_3 _locationy_3) (Game|Player|GetMousePosition _returnvalue))
  (return (Math|Vector2D|Vector2DLength (select (Utilities|Enum|Equal(Enum) (Game|GetPlatformName) "Windows") (Math|Vector2D|MakeVector2D _locationx_3 _locationy_3) (- (Math|Vector2D|MakeVector2D _locationx_2 _locationy_2) (Math|Vector2D|MakeVector2D _locationx _locationy))))))